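; Infinite terrain game mode that spawns chained BP_Tile actors and counts conquered tiles.
; On BeginPlay it populates a NavMesh bounds volume pool, then spawns an initial tile.
; Each spawned tile receives that pool and supplies its attach location as the transform for the next spawn.
; IncrementScore raises the TileConquered count and prints it.
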(event `self.ReceiveBeginPlay`
  (`self.PopulateBoundsVolumePool`)
  (for _ (range 1)
    (`self.Spawn Terrain`)))

(fn `IncrementScore`
  (bind _result (`/Engine/EditorBlueprintResources/StandardMacros.IncrementInt` (`self.TileConquered`))
    (:`  `
      (`KismetSystemLibrary.PrintString` (`KismetStringLibrary.Conv_IntToString` _result)))))

(fn `Spawn Terrain`
  (bind _returnvalue (`|SpawnActorFromClass` "/Game/Blueprints/Terrain/BP_Tile.BP_Tile_C" (`self.SpawnTransform`) "Undefined" "OverrideRootScale" null (`GameplayStatics.GetPlayerPawn` 0)))
  (`Tile.SetPool` _returnvalue (`self.NavMeshBoundsVolumePool`))
  (bind _attachtransform (`/Game/Blueprints/Terrain/BP_Tile.Get Attach Location` _returnvalue))
  (set `self.SpawnTransform` _attachtransform))

(fn `UserConstructionScript`)