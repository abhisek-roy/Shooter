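; BP_ShooterPlayerController is the shooter's player controller and handles opening the pause menu.
; It creates WBP_PauseMenu once at BeginPlay and stores it in PauseMenuObject, which GetPauseObject returns.
; Releasing the Pause input pauses the game, adds the stored menu to the viewport, shows the cursor and switches to UI-only input focused on the menu.
; It contains no resume logic.
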(event `self.ReceiveBeginPlay`
  (bind _returnvalue (`|CreateWidget` "/Game/Blueprints/UI/WBP_PauseMenu.WBP_PauseMenu_C"))
  (set `self.PauseMenuObject` _returnvalue))

(event `InputAction|Pause`
  (params (Key :type "Key Structure"))
  (:`Released`
    (`GameplayStatics.SetGamePaused` true)
    (bind _aswbp_pause_menu (cast `/Game/Blueprints/UI/WBP_PauseMenu` (`self.PauseMenuObject`)))
    (`UserWidget.AddToViewport` _aswbp_pause_menu 0)
    (set `self.bShowMouseCursor` true)
    (`WidgetBlueprintLibrary.SetInputMode_UIOnlyEx` self _aswbp_pause_menu)))

(fn `GetPauseObject`
  (returns (PauseMenuObject :type "Object Object Reference"))
  (return (`self.PauseMenuObject`)))

(fn `UserConstructionScript`)