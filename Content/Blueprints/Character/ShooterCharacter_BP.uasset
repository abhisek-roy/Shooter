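; Shooter character Blueprint that adds health feedback and a gate-crossing screen effect to player and AI characters.
; Each Tick fades in the low-health effect's blend weight as health drops below a quarter, clearing it at zero.
; AI-controlled characters show an updated health bar widget while they have line of sight to the player; others hide it.
; PlayGateCrossingVFX runs a timeline that drives the gate-crossing effect's blend weight.
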(event `PlayGateCrossingVFX`
  (bind (_direction _blend) (`Timeline|VFX Blend` :!via `PlayFromStart`)
    (:`Update`
      (set `PostProcessComponent.BlendWeight` _blend (`self.GateCrossingVFX`)))))

(event `self.ReceiveTick`
  (params (DeltaSeconds :type "Float (single-precision)"))
  (`self.ShowLowHealth`)
  (bind _asaicontroller (cast `AIController` (`self.GetController`))
    (:`then`
      (`self.ShowHealthBarWhenVisible` _asaicontroller))
    (:`CastFailed`
      ;[1 1 1] Hide HealthBar for Player
      (`SceneComponent.SetVisibility` (`self.W_HealthBar`) false false))))

(fn `ShowHealthBarWhenVisible`
  (params (self2 :type "Controller Object Reference"))
  (bind _w_healthbar (`self.W_HealthBar`))
  (`SceneComponent.SetVisibility` _w_healthbar (`Controller.LineOfSightTo` self2 (`GameplayStatics.GetPlayerPawn` 0) (0.0 0.0 0.0) false) false)
  (bind _aswbp_health_bar (cast `/Game/Blueprints/UI/WBP_HealthBar` (`WidgetComponent.GetWidget` _w_healthbar)))
  (`/Game/Blueprints/UI/WBP_HealthBar.SetHealth` _aswbp_health_bar (`self.GetHealthPercent`)))

(fn `ShowLowHealth`
  (bind _returnvalue (`self.GetHealthPercent`))
  (set `PostProcessComponent.BlendWeight` (`KismetMathLibrary.SelectFloat` (- 1.0 (* (`KismetMathLibrary.FClamp` _returnvalue 0.0 0.25) 4.0)) 0.0 (> _returnvalue 0.0)) (`self.LowHealthVFX`)))

(fn `UserConstructionScript`)