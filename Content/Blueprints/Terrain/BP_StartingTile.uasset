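; BP_StartingTile is a terrain tile that fills itself with props and AI shooter enemies on BeginPlay.
; PlaceActors scatters containers, rocks, boxes, sacks and canisters by count, radius and scale, while PlaceAIPawns spawns enemies.
; A gate starts locked red, turns green and passable on player overlap, then relocks with crossing VFX.
; An Arrow supplies the attach transform, and the tile destroys itself when the player exits UnloadTile.
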(event `self.ReceiveBeginPlay`
  (`self.Lock`)
  (`|ExecutionSequence`
    (:`then_0`
      (`self.PlaceActors` "/Game/Blueprints/Terrain/BP_Container.BP_Container_C" 1 2 500.0)
      (`self.PlaceActors` "/Game/Blueprints/Terrain/BP_Rock3.BP_Rock3_C" 0 1 275.0 4.0 3.0)
      (`self.PlaceActors` "/Game/Blueprints/Terrain/BP_Rock2.BP_Rock2_C" 2 1 150.0 1.5)
      (`self.PlaceActors` "/Game/Blueprints/Terrain/BP_Box.BP_Box_C" 5 6 100.0))
    (:`then_1`
      (`self.PlaceActors` "/Game/Blueprints/Terrain/BP_Sacks.BP_Sacks_C" 3 5 200.0 1.0 1.5)
      (`self.PlaceActors` "/Game/Blueprints/Terrain/BP_Canister.BP_Canister_C" 5 10 50.0)
      (`self.PlaceActors` "/Game/Blueprints/Terrain/BP_Rock1.BP_Rock1_C" 10 20 150.0 0.4 0.2)
      (`self.PlaceAIPawns` "/Game/Blueprints/Character/ShooterCharacter_BP.ShooterCharacter_BP_C" (`self.MinEnemies`) (`self.MaxEnemies`)))))

(event `self.GatingMechanism.OnComponentBeginOverlap`
  (params (OverlappedComponent :type "PrimitiveComponent Object Reference") (OtherActor :type "Actor Object Reference") (OtherComp :type "PrimitiveComponent Object Reference") (OtherBodyIndex :type Integer) (bFromSweep :type Boolean) (SweepResult :type "HitResult Structure (by ref)"))
  (`self.IsPlayer` OtherActor)
  (`self.Unlock`))

(event `self.GatingMechanism.OnComponentEndOverlap`
  (params (OverlappedComponent :type "PrimitiveComponent Object Reference") (OtherActor :type "Actor Object Reference") (OtherComp :type "PrimitiveComponent Object Reference") (OtherBodyIndex :type Integer))
  (`self.IsPlayer` OtherActor)
  (`|ExecutionSequence`
    (:`then_0`
      (`self.Lock`))
    (:`then_1`
      (bind _asshooter_character_bp (cast `/Game/Blueprints/Character/ShooterCharacter_BP` OtherActor))
      (`/Game/Blueprints/Character/ShooterCharacter_BP.PlayGateCrossingVFX` _asshooter_character_bp))))

(event `self.UnloadTile.OnComponentEndOverlap`
  (params (OverlappedComponent :type "PrimitiveComponent Object Reference") (OtherActor :type "Actor Object Reference") (OtherComp :type "PrimitiveComponent Object Reference") (OtherBodyIndex :type Integer))
  (`self.IsPlayer` OtherActor)
  (`self.K2_DestroyActor`))

(fn `Get Attach Location`
  (returns (AttachTransform :type "Transform Structure"))
  (return (`SceneComponent.K2_GetComponentToWorld` (`self.Arrow`))))

(fn `Lock`
  (`PrimitiveComponent.SetCollisionEnabled` (`self.Gate`) "QueryAndPhysics")
  (`PrimitiveComponent.SetMaterial` (`self.Gate`) 0 "/Game/Levels/Terrain/Materials/MI_Barrier_Red.MI_Barrier_Red"))

(fn `Unlock`
  (`PrimitiveComponent.SetCollisionEnabled` (`self.Gate`) "NoCollision")
  (`PrimitiveComponent.SetMaterial` (`self.Gate`) 0 "/Game/Levels/Terrain/Materials/MI_Barrier_Green.MI_Barrier_Green"))

(fn `UserConstructionScript`
  (`self.Lock`))