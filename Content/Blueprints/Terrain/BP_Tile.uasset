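; BP_Tile is a segment of endless terrain that scatters props on itself and gates the player's progress.
; On BeginPlay it locks the gate and calls PlaceActors for containers, boxes, sacks and rocks, with randomized count ranges.
; The player entering GatingMechanism asks InfiniteTerrainMode to spawn terrain and unlocks the gate (green, no collision); leaving relocks it.
; Exiting UnloadTile destroys the tile, while GetAttachLocation exposes the Arrow's transform as an attach point.
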(event `self.ReceiveBeginPlay`
  (`self.Lock`)
  (`self.PlaceActors` "/Game/Blueprints/Terrain/BP_Container.BP_Container_C" 2 3 500.0)
  (`self.PlaceActors` "/Game/Blueprints/Terrain/BP_Box.BP_Box_C" 5 6 100.0)
  (`self.PlaceActors` "/Game/Blueprints/Terrain/BP_Sacks.BP_Sacks_C" 3 5 200.0)
  (`self.PlaceActors` "/Game/Blueprints/Terrain/BP_Rock1.BP_Rock1_C" 10 20 150.0)
  (`self.PlaceActors` "/Game/Blueprints/Terrain/BP_Rock2.BP_Rock2_C" 10 15 150.0)
  (`self.PlaceActors` "/Game/Blueprints/Terrain/BP_Rock3.BP_Rock3_C" 10 15 275.0))

(event `self.GatingMechanism.OnComponentBeginOverlap`
  (params (OverlappedComponent :type "PrimitiveComponent Object Reference") (OtherActor :type "Actor Object Reference") (OtherComp :type "PrimitiveComponent Object Reference") (OtherBodyIndex :type Integer) (bFromSweep :type Boolean) (SweepResult :type "HitResult Structure (by ref)"))
  (`self.IsPlayer` OtherActor)
  (bind _asinfinite_terrain_mode (cast `/Game/Blueprints/InfiniteTerrainMode` (`GameplayStatics.GetGameMode`)))
  (`/Game/Blueprints/InfiniteTerrainMode.Spawn Terrain` _asinfinite_terrain_mode)
  (`self.Unlock`))

(event `self.GatingMechanism.OnComponentEndOverlap`
  (params (OverlappedComponent :type "PrimitiveComponent Object Reference") (OtherActor :type "Actor Object Reference") (OtherComp :type "PrimitiveComponent Object Reference") (OtherBodyIndex :type Integer))
  (`self.IsPlayer` OtherActor)
  (`self.Lock`))

(event `self.UnloadTile.OnComponentEndOverlap`
  (params (OverlappedComponent :type "PrimitiveComponent Object Reference") (OtherActor :type "Actor Object Reference") (OtherComp :type "PrimitiveComponent Object Reference") (OtherBodyIndex :type Integer))
  (`self.IsPlayer` OtherActor)
  (`self.K2_DestroyActor`))

(fn `Get Attach Location`
  (returns (AttachTransform :type "Transform Structure"))
  (return (`SceneComponent.K2_GetComponentToWorld` (`self.Arrow`))))

(fn `Lock`
  (`PrimitiveComponent.SetCollisionEnabled` (`self.Gate`) "QueryAndPhysics")
  (`PrimitiveComponent.SetMaterial` (`self.Gate`) 0 "/Game/Levels/Terrain/Materials/MI_Barrier_Red.MI_Barrier_Red"))

(fn `Unlock`
  (`PrimitiveComponent.SetCollisionEnabled` (`self.Gate`) "NoCollision")
  (`PrimitiveComponent.SetMaterial` (`self.Gate`) 0 "/Game/Levels/Terrain/Materials/MI_Barrier_Green.MI_Barrier_Green"))

(fn `UserConstructionScript`
  (`self.Lock`))